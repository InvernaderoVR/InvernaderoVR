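; BP_FruitContainer is a sales-order container that counts the fruit actors inside its Box volume and can remove requested amounts of them.
; On BeginPlay and every overlap change it rescans the box, broadcasting reset, per-fruit identifier and show events through dispatchers for listeners to tally.
; DeleteFruits takes an array of counts indexed by fruit identifier, destroying matching overlapping fruits and decrementing each count until it reaches zero.
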(event `self.ReceiveBeginPlay`
  (`self.Refresh Quantities`))

(event `self.Box.OnComponentBeginOverlap`
  (params (OverlappedComponent :type "PrimitiveComponent Object Reference") (OtherActor :type "Actor Object Reference") (OtherComp :type "PrimitiveComponent Object Reference") (OtherBodyIndex :type Integer) (bFromSweep :type Boolean) (SweepResult :type "HitResult Structure (by ref)"))
  (`self.Refresh Quantities`))

(event `self.Box.OnComponentEndOverlap`
  (params (OverlappedComponent :type "PrimitiveComponent Object Reference") (OtherActor :type "Actor Object Reference") (OtherComp :type "PrimitiveComponent Object Reference") (OtherBodyIndex :type Integer))
  (`self.Refresh Quantities`))

(event `Refresh Quantities`
  (`self.ResetQuantities`)
  (for _array_element (`PrimitiveComponent.GetOverlappingActors` (`self.Box`) "/Game/Blueprints/BP_Fruits/BP_Fruit.BP_Fruit_C")
    (bind _asbp_fruit (cast `/Game/Blueprints/BP_Fruits/BP_Fruit` _array_element))
    (bind (_fruitdata_fruitname _fruitdata_fruitidentificator) (break `/Game/Blueprints/BP_Fruits/F_Fruit` (`/Game/Blueprints/BP_Fruits/BP_Fruit.FruitData` _asbp_fruit)))
    (`self.SendData` _fruitdata_fruitidentificator))
  (`self.ShowData`))

(event `DeleteFruits`
  (params (FruitsToDelete :type "Array of Integer"))
  (for _array_element (`PrimitiveComponent.GetOverlappingActors` (`self.Box`) "/Game/Blueprints/BP_Fruits/BP_Fruit.BP_Fruit_C")
    (bind _asbp_fruit (cast `/Game/Blueprints/BP_Fruits/BP_Fruit` _array_element))
    (bind (_fruitdata_fruitname _fruitdata_fruitidentificator) (break `/Game/Blueprints/BP_Fruits/F_Fruit` (`/Game/Blueprints/BP_Fruits/BP_Fruit.FruitData` _asbp_fruit)))
    (bind _output (`|GetArrayItem` FruitsToDelete _fruitdata_fruitidentificator))
    (if (> _output 0)
      (bind _result (`/Engine/EditorBlueprintResources/StandardMacros.DecrementInt` _output)
        (:`  `
          (`KismetArrayLibrary.Array_Set` FruitsToDelete _fruitdata_fruitidentificator _result)
          (`self.K2_DestroyActor` _array_element))))))

(fn `UserConstructionScript`)